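; Attack component for BP_TopDownCharacter that runs a four-hit great sword combo from the IA_Attack input.
; Each press plays the montage for the current ComboCounter on the character mesh, with IsAttack blocking further presses.
; A montage notify clears the lock and advances the counter, wrapping after the fourth hit.
; Each swing also sets a one-second timer, counted from montage start, that resets the combo to the first hit.
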(event Custom|ResetCounter
  (Variables|Default|SetCombo%20Counter 0))

(event Input|EnhancedActionEvents|EnhancedInputActionIA_Attack
  (params (ActionValue :type Boolean) (ElapsedSeconds :type Float%20%28double-precision%29) (TriggeredSeconds :type Float%20%28double-precision%29) (InputAction :type Input%20Action%20Object%20Reference :default "/Game/LJY/Input/IA_Attack.IA_Attack"))
  (bind _character_mesh (Variables|Default|GetCharacter%20Mesh))
  (if (not (Variables|Default|Getis%20Attack))
    (Variables|Default|Setis%20Attack true)
    (switch int (Variables|Default|GetCombo%20Counter)
      (:0
        (Animation|Montage|PlayMontage _character_mesh "/Game/LJY/Animation/Great_Sword_Pack/slashMontage/great_sword_slash_Montage.great_sword_slash_Montage"
          (:then
            (Utilities|Time|SetTimerbyEvent (delegate Custom|ResetCounter) 1.0 :!label _label))
          (:OnNotifyBegin
            (Variables|Default|Setis%20Attack false)
            (Variables|Default|SetCombo%20Counter 1))))
      (:1
        (Animation|Montage|PlayMontage _character_mesh "/Game/LJY/Animation/Great_Sword_Pack/slashMontage/great_sword_slash__3__Montage.great_sword_slash__3__Montage"
          (:then
            (goto _label))
          (:OnNotifyBegin
            (Variables|Default|Setis%20Attack false)
            (Variables|Default|SetCombo%20Counter 2))))
      (:2
        (Animation|Montage|PlayMontage _character_mesh "/Game/LJY/Animation/Great_Sword_Pack/slashMontage/great_sword_slash__4__Montage.great_sword_slash__4__Montage"
          (:then
            (goto _label))
          (:OnNotifyBegin
            (Variables|Default|Setis%20Attack false)
            (Variables|Default|SetCombo%20Counter 3))))
      (:3
        (Animation|Montage|PlayMontage _character_mesh "/Game/LJY/Animation/Great_Sword_Pack/slashMontage/great_sword_slash__5__Montage.great_sword_slash__5__Montage"
          (:then
            (goto _label))
          (:OnNotifyBegin
            (Variables|Default|Setis%20Attack false)
            (Variables|Default|SetCombo%20Counter 0)))))))

(event EventBeginPlay
  (bind _asbp_top_down_character (Utilities|Casting|CastToBP_TopDownCharacter (Components|GetOwner)))
  (bind _output_get (Variables|Default|SetAs%20BP%20Top%20Down%20Character _asbp_top_down_character))
  (Variables|Default|SetCharacter%20Mesh (Variables|/Script/Engine.Character|GetMesh _output_get)))

(event EventTick
  (params (DeltaSeconds :type Float%20%28single-precision%29)))